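; Mesh component for a holographic aircraft HUD, rendered through a dynamic instance of M_Hud2.
; BeginPlay applies display, hologram and glass settings to the material, then binds to HUD updates.
; Updates feed scaled roll, pitch and yaw into material parameters; altitude, speed and flight path are unused.
; A 512x512 canvas render target supplies a material texture, drawn with hard-coded placeholder text and refreshed only at BeginPlay.
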(event Custom|Hud_Update_Event
  (params (Roll :type Float%20%28single-precision%29) (Pitch :type Float%20%28single-precision%29) (Yaw :type Float%20%28single-precision%29) (Altitude :type Float%20%28single-precision%29) (Speed :type Float%20%28single-precision%29) (FlightPath :type Vector))
  (bind _mid_hud (Variables|Default|GetMID_Hud))
  (Utilities|IsValid _mid_hud
    (:Is%20Valid
      (Rendering|Material|SetScalarParameterValue _mid_hud "Roll" (/ Roll 3.6e+02) :!class /Script/Engine.MaterialInstanceDynamic)
      (Rendering|Material|SetScalarParameterValue _mid_hud "Pitch" (* Pitch 0.004167) :!class /Script/Engine.MaterialInstanceDynamic)
      (Rendering|Material|SetScalarParameterValue _mid_hud "Heading" (/ Yaw 3.6e+02) :!class /Script/Engine.MaterialInstanceDynamic))))

(event Custom|Event_DrawText
  (params (Canvas :type Canvas%20Object%20Reference) (Width :type Integer) (Height :type Integer))
  (Canvas|DrawTexture :self Canvas :ScreenSize (Math|Vector2D|MakeVector2D (Math|Conversions|ToFloat(Integer) Width) (Math|Conversions|ToFloat(Integer) Height)) :RenderColor "(R=1.000000,G=0.000000,B=0.000000,A=0.000000)")
  (HUD|DrawText Canvas "/Engine/EngineFonts/TinyFont.TinyFont" "Hiho das ist ein Text" "(X=500.000000,Y=500.000000)" "(R=255.000000,G=0.000000,B=0.000000,A=1.000000)" 0.0 "(R=0.000000,G=0.000000,B=0.000000,A=1.000000)" "(X=1.000000,Y=1.000000)" true true false "(R=0.000000,G=0.000000,B=0.000000,A=1.000000)"))

(event EventBeginPlay
  (bind _returnvalue (Rendering|Material|CreateDynamicMaterialInstance 0 "/Game/AircraftHud/M_Hud2.M_Hud2" :!class /Script/Engine.PrimitiveComponent))
  (bind _output_get (Variables|Default|SetMID_Hud _returnvalue))
  (Rendering|Material|SetMaterial 0 _output_get)
  (Rendering|Material|SetScalarParameterValue (Variables|Default|GetMID_Hud) "BumpDistance" (Variables|Default|GetDisplayDistance) :!class /Script/Engine.MaterialInstanceDynamic)
  (Rendering|Material|SetScalarParameterValue (Variables|Default|GetMID_Hud) "BumpScale" (Variables|Default|GetDisplayScale) :!class /Script/Engine.MaterialInstanceDynamic)
  (Rendering|Material|SetVectorParameterValue (Variables|Default|GetMID_Hud) "HologramColor" (Math|Conversions|ToLinearColor(Color) (Variables|Default|GetHologramColor)) :!class /Script/Engine.MaterialInstanceDynamic)
  (Rendering|Material|SetScalarParameterValue (Variables|Default|GetMID_Hud) "HologramStrength" (Variables|Default|GetHologramIntensity) :!class /Script/Engine.MaterialInstanceDynamic)
  (Rendering|Material|SetVectorParameterValue (Variables|Default|GetMID_Hud) "GlassColor" (Math|Conversions|ToLinearColor(Color) (Variables|Default|GetGlassColor)) :!class /Script/Engine.MaterialInstanceDynamic)
  (Rendering|Material|SetScalarParameterValue (Variables|Default|GetMID_Hud) "GlassOpacity" (Variables|Default|GetGlassOpacity) :!class /Script/Engine.MaterialInstanceDynamic)
  (EventDispatchers|BindEventtoHudUpdate (delegate Custom|Hud_Update_Event))
  (bind _returnvalue_2 (CanvasRenderTarget2D|CreateCanvasRenderTarget2D "/Script/Engine.CanvasRenderTarget2D" 512 512))
  (bind _output_get_2 (Variables|Default|SetTextRenderTexture _returnvalue_2))
  (Rendering|Material|SetTextureParameterValue (Variables|Default|GetMID_Hud) "TP2D" (Variables|Default|GetTextRenderTexture))
  (EventDispatchers|BindEventtoOnCanvasRenderTargetUpdate _output_get_2 (delegate Custom|Event_DrawText))
  (Class|CanvasRenderTarget2D|UpdateResource _output_get_2))

(event EventTick
  (params (DeltaSeconds :type Float%20%28single-precision%29)))