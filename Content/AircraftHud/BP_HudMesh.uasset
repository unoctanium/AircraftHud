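; Aircraft HUD mesh that displays a holographic pitch ladder on glass through a dynamic instance of M_Hud.
; On BeginPlay it pushes display distance, scale, tiling, hologram and glass settings into the material, then binds to the HUD update event.
; Each update pans the pitch ladder in the material from Pitch, offset by its vertical tiling.
; Roll, yaw, altitude, speed and flight path arrive with the event but are unused.
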(event Custom|Hud_Update_Event
  (params (Roll :type Float%20%28single-precision%29) (Pitch :type Float%20%28single-precision%29) (Yaw :type Float%20%28single-precision%29) (Altitude :type Float%20%28single-precision%29) (Speed :type Float%20%28single-precision%29) (FlightPath :type Vector))
  (bind _mid_hud (Variables|Default|GetMID_Hud))
  (Utilities|IsValid _mid_hud
    (:Is%20Valid
      (Rendering|Material|SetScalarParameterValue _mid_hud "PitchLadderPan" (- (- 0.5 (/ (Variables|Default|GetPitchLadderVTile) 2.0)) (/ (/ Pitch 9e+01) 3.0)) :!class /Script/Engine.MaterialInstanceDynamic))))

(event EventBeginPlay
  (bind _returnvalue (Rendering|Material|CreateDynamicMaterialInstance 0 "/Game/AircraftHud/M_Hud.M_Hud" :!class /Script/Engine.PrimitiveComponent))
  (bind _output_get (Variables|Default|SetMID_Hud _returnvalue))
  (Rendering|Material|SetMaterial 0 _output_get)
  (Rendering|Material|SetScalarParameterValue (Variables|Default|GetMID_Hud) "PitchladderVTile" (Variables|Default|GetPitchLadderVTile) :!class /Script/Engine.MaterialInstanceDynamic)
  (Rendering|Material|SetScalarParameterValue (Variables|Default|GetMID_Hud) "BumpDistance" (Variables|Default|GetDisplayDistance) :!class /Script/Engine.MaterialInstanceDynamic)
  (Rendering|Material|SetScalarParameterValue (Variables|Default|GetMID_Hud) "BumpScale" (Variables|Default|GetDisplayScale) :!class /Script/Engine.MaterialInstanceDynamic)
  (Rendering|Material|SetVectorParameterValue (Variables|Default|GetMID_Hud) "HologramColor" (Math|Conversions|ToLinearColor(Color) (Variables|Default|GetHologramColor)) :!class /Script/Engine.MaterialInstanceDynamic)
  (Rendering|Material|SetScalarParameterValue (Variables|Default|GetMID_Hud) "HologramStrength" (Variables|Default|GetHologramIntensity) :!class /Script/Engine.MaterialInstanceDynamic)
  (Rendering|Material|SetVectorParameterValue (Variables|Default|GetMID_Hud) "GlassColor" (Math|Conversions|ToLinearColor(Color) (Variables|Default|GetGlassColor)) :!class /Script/Engine.MaterialInstanceDynamic)
  (Rendering|Material|SetScalarParameterValue (Variables|Default|GetMID_Hud) "GlassOpacity" (Variables|Default|GetGlassOpacity) :!class /Script/Engine.MaterialInstanceDynamic)
  (EventDispatchers|BindEventtoHudUpdate (delegate Custom|Hud_Update_Event)))

(event EventTick
  (params (DeltaSeconds :type Float%20%28single-precision%29)))