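; Aircraft HUD mesh that displays flight data entirely through a dynamic material.
; BeginPlay creates the material instance and binds to a HUD update event, whose values are written to scalar parameters for attitude, speed, altitude, trend lines, skid and flight path.
; Attitude and flight path values are scaled into material units.
; Speed and altitude are split into five per-digit parameters, with a special leading-digit value for negatives.
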(event Custom|Hud_Update_Event
  (params (Roll :type Float%20%28single-precision%29) (Pitch :type Float%20%28single-precision%29) (Yaw :type Float%20%28single-precision%29) (Altitude :type Float%20%28single-precision%29) (Speed :type Float%20%28single-precision%29) (DeltaSpeed :type Float%20%28single-precision%29) (DeltaAlt :type Float%20%28single-precision%29) (Skid :type Float%20%28single-precision%29) (FlightPathUp :type Float%20%28single-precision%29) (FlightPathRight :type Float%20%28single-precision%29))
  (|SetAttitudeMaterialParameters Roll Pitch Yaw)
  (|SetAltDigitsMaterialParameters Altitude)
  (|SetSpeedDigitsMaterialParameters Speed)
  (|SetDeltaLinesMaterialParameters DeltaSpeed DeltaAlt)
  (Rendering|Material|SetScalarParameterValue (Variables|Default|GetMID_Hud) "SkidPercent" Skid :!class /Script/Engine.MaterialInstanceDynamic)
  (|SetFlightPathMaterialParametrers FlightPathRight FlightPathUp))

(event EventBeginPlay
  (bind _returnvalue (Rendering|Material|CreateDynamicMaterialInstance 0 (Variables|Default|GetHudMaterial) :!class /Script/Engine.PrimitiveComponent))
  (bind _output_get (Variables|Default|SetMID_Hud _returnvalue))
  (Rendering|Material|SetMaterial 0 _output_get)
  (EventDispatchers|BindEventtoHudUpdate (delegate Custom|Hud_Update_Event)))

(event EventTick
  (params (DeltaSeconds :type Float%20%28single-precision%29)))